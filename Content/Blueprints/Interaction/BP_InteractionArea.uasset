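; BP_InteractionArea is an interaction helper that relays focus changes to the actor it is attached to as a child actor.
; ToggleFocus stores the Focused state and forwards it to the parent actor through an interface message.
; It then gets the parent's interaction widget through another interface message, shows it only while focused, and prints the state for debugging.
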(event Custom|ToggleFocus
  (params (Focused :type Boolean))
  (Variables|Default|SetFocused Focused)
  (Class|BIInteraction|InterfaceToggleFocus(Message) (Actor|GetParentActor) (Variables|Default|GetFocused))
  (bind _ref (Class|BIInteraction|GetInteractionWidgetRef(Message) (Actor|GetParentActor)))
  (Development|SetHiddeninGame _ref (not (Variables|Default|GetFocused)) false)
  (Development|PrintString (Utilities|String|ToString(Boolean) (Variables|Default|GetFocused))))

(fn ConstructionScript)