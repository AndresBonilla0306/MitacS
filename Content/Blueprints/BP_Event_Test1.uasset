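; BP_Event_Test1 is an interactable event object that highlights a cube on focus through custom depth and exposes a pop-up widget showing configurable text and image.
; Interaction calls InteracOnServer to flip InteractToggle, whose RepNotify plays the Daft sound and adds a new WI_Event screen widget with text, image and description on every toggle, regardless of value.
; StopSound halts the audio.
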(event Custom|InteracOnServer
  (Variables|Default|SetInteractToggle (not (Variables|Default|GetInteractToggle))))

(event EventInterfaceToggleFocus
  (params (Focus :type Boolean))
  (Rendering|SetRenderCustomDepth (Variables|Default|GetCubeEvent) Focus))

(event EventBeginPlay
  (Audio|Components|Audio|SetSound (Variables|Default|GetDaft) (Variables|Default|GetPopAudio))
  (bind _asbp_popo_up (Utilities|Casting|CastToBP_PopoUp (UserInterface|GetUserWidgetObject (Variables|Default|GetWidget))))
  (Variables|/Game/Blueprints/Interaction/BP_PopoUp.BP_PopoUp_C|SetPopUpText _asbp_popo_up (Variables|Default|GetPopText))
  (Variables|/Game/Blueprints/Interaction/BP_PopoUp.BP_PopoUp_C|SetPopUpTexture _asbp_popo_up (Variables|Default|GetPopImage))
  (Variables|Default|SetEventTestRef (Variables|Default|GetEventTestRef)))

(event EventInterfaceInteract
  (CallFunction|InteraconServer))

(fn ConstructionScript)

(fn OnRepInteractToggle
  (Audio|Components|Audio|Play (Variables|Default|GetDaft) 0.0)
  (bind _returnvalue (UserInterface|CreateWidget "/Game/Blueprints/Interaction/WI_Event.WI_Event_C"))
  (bind _output_get (Variables|Default|SetWEventReference _returnvalue))
  (Variables|/Game/Blueprints/Interaction/WI_Event.WI_Event_C|SetPopUpText _output_get (Variables|Default|GetPopText))
  (Variables|/Game/Blueprints/Interaction/WI_Event.WI_Event_C|SetPopUpTexture _output_get (Variables|Default|GetPopImage))
  (Variables|/Game/Blueprints/Interaction/WI_Event.WI_Event_C|SetPopUpDesc _output_get (Variables|Default|GetPopUpDesc))
  (UserInterface|Viewport|AddtoViewport _output_get 0))

(fn StopSound
  (Development|PrintString "Stopping" true true "(R=1.000000,G=0.000000,B=0.931750,A=1.000000)")
  (Audio|Components|Audio|Stop (Variables|Default|GetDaft)))

(fn GetInteractionWidgetRef
  (return (Variables|Default|GetWidget)))